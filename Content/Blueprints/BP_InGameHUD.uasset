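; BP_InGameHUD creates and manages the in-game UI: an item overlap alert, the main interface and an inventory widget.
; BeginPlay creates all three for player 0 and adds them to the viewport, with the alert and inventory starting hidden.
; AlertWidgetOn shows the alert with the item's name from the supplied data, and AlertWidgetOff hides it.
; RefreshWidget forwards to the inventory widget's Refresh without changing its visibility.
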(event EventBeginPlay
  (bind _returnvalue (UserInterface|CreateWidget "/Game/Blueprints/WBP_ItemOverlapAlert.WBP_ItemOverlapAlert_C" (Game|GetPlayerController 0)))
  (bind _output_get (Variables|Default|SetAlertWidget _returnvalue))
  (Widget|SetVisibility (Variables|Default|GetAlertWidget) "Hidden")
  (UserInterface|Viewport|AddtoViewport _returnvalue 0)
  (bind _returnvalue_2 (UserInterface|CreateWidget "/Game/Blueprints/WBP_Interface.WBP_Interface_C" (Game|GetPlayerController 0)))
  (UserInterface|Viewport|AddtoViewport _returnvalue_2 0)
  (bind _returnvalue_3 (UserInterface|CreateWidget "/Game/Blueprints/WBP_InventoryWidget.WBP_InventoryWidget_C" (Game|GetPlayerController 0)))
  (Variables|Default|SetInventoryWidget _returnvalue_3)
  (UserInterface|Viewport|AddtoViewport _returnvalue_3 0)
  (Widget|SetVisibility _returnvalue_3 "Hidden"))

(event EventTick
  (params (DeltaSeconds :type Float%20%28single-precision%29)))

(fn ConstructionScript)

(fn AlertWidgeton
  (params (ItemData :type Inventory%20Data%20Structure))
  (bind _alertwidget (Variables|Default|GetAlertWidget))
  (Widget|SetVisibility _alertwidget "Visible")
  (Rendering|Components|TextRender|SetText (Variables|/Game/Blueprints/WBP_ItemOverlapAlert.WBP_ItemOverlapAlert_C|GetAlertText _alertwidget) (Utilities|Text|ToText(String) (.itemname ItemData))))

(fn AlertWidgetOff
  (Widget|SetVisibility (Variables|Default|GetAlertWidget) "Hidden"))

(fn RefreshWidget
  (Default|Refresh (Variables|Default|GetInventoryWidget)))