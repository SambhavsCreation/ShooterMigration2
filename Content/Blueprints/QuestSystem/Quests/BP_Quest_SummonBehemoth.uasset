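; BP_Quest_SummonBehemoth is a quest in which the player summons the behemoth at a summoning area.
; It overrides the parent quest's hooks to build an ordered root objective collection holding a single BP_OBJSummonBehemoth objective, which receives the SummoningArea reference.
; SetupPOI sets that same area as the quest's point-of-interest target before running the parent setup.
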(fn ConstructionScript
  (|CallParentFunction))

(fn PopulateObjectives
  (params (RootObjectiveCollection :type BP%20OBJ%20Collection%20Object%20Reference))
  (bind _self self)
  (bind _returnvalue (Game|ConstructObjectfromClass "/Game/Blueprints/QuestSystem/Objectives/BP_OBJSummonBehemoth.BP_OBJSummonBehemoth_C" _self (Variables|Default|GetSummoningArea) "Summon the behemoth" _self))
  (Default|AddObjective RootObjectiveCollection _returnvalue))

(fn ConstructRootObjectiveCollection
  (bind _self self)
  (bind _returnvalue (Game|ConstructObjectfromClass "/Game/Blueprints/QuestSystem/Objectives/BP_OBJCollection.BP_OBJCollection_C" _self true "Summon the behemoth" _self))
  (return _returnvalue))

(fn SetupPOI
  (Variables|Default|SetTarget (Variables|Default|GetSummoningArea))
  (|CallParentFunction))