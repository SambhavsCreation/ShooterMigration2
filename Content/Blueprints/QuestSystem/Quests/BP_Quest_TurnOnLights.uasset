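; Quest Blueprint for "Light a path", in which the objective is to turn on lights.
; It overrides the quest base's construction hooks to create an order-required root objective collection and add a single turn-on-light objective bound to its Lights variable.
; POI setup assigns Lights as the target before running the parent logic; the event graph holds only disabled default events.
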(event EventBeginPlay
  (|CallParentFunction) ; This node is disabled and will not be called.\nDrag off pins to build functionality.
)

(event Collision|EventActorBeginOverlap
  (params (OtherActor :type Actor%20Object%20Reference))
  (|CallParentFunction OtherActor) ; This node is disabled and will not be called.\nDrag off pins to build functionality.
)

(event EventTick
  (params (DeltaSeconds :type Float%20%28single-precision%29))
  (|CallParentFunction DeltaSeconds) ; This node is disabled and will not be called.\nDrag off pins to build functionality.
)

(fn ConstructionScript
  (|CallParentFunction))

(fn ConstructRootObjectiveCollection
  (bind _self self)
  (bind _returnvalue (Game|ConstructObjectfromClass "/Game/Blueprints/QuestSystem/Objectives/BP_OBJCollection.BP_OBJCollection_C" _self true "Light a path" _self))
  (return _returnvalue))

(fn PopulateObjectives
  (params (RootObjectiveCollection :type BP%20OBJ%20Collection%20Object%20Reference))
  (bind _self self)
  (bind _returnvalue (Game|ConstructObjectfromClass "/Game/Blueprints/QuestSystem/Objectives/BP_OBJTurnOnLight.BP_OBJTurnOnLight_C" _self (Variables|Default|GetLights) (Utilities|String|MakeLiteralString "Turn On Light") _self))
  (Default|AddObjective RootObjectiveCollection _returnvalue))

(fn SetupPOI
  (Variables|Default|SetTarget (Variables|Default|GetLights))
  (|CallParentFunction))