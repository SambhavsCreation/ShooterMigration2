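; BP_Quest_4 is a quest in the quest system that tasks the player with picking up an AKM rifle.
; It builds an ordered root objective collection named PickUpRifle, then adds a single BP_PickUpAKM objective bound to the AKM reference.
; POI setup sets the AKM as the target before running the parent's logic.
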(fn ConstructionScript
  (|CallParentFunction))

(fn ConstructRootObjectiveCollection
  (bind _self self)
  (bind _returnvalue (Game|ConstructObjectfromClass "/Game/Blueprints/QuestSystem/Objectives/BP_OBJCollection.BP_OBJCollection_C" _self true "PickUpRifle" _self))
  (return _returnvalue))

(fn PopulateObjectives
  (params (RootObjectiveCollection :type BP%20OBJ%20Collection%20Object%20Reference))
  (bind _self self)
  (bind _returnvalue (Game|ConstructObjectfromClass "/Game/Blueprints/QuestSystem/Objectives/BP_PickUpAKM.BP_PickUpAKM_C" _self (Variables|Default|GetAKM) "PickUpAKM" _self))
  (Default|AddObjective RootObjectiveCollection _returnvalue))

(fn SetupPOI
  (Variables|Default|SetTarget (Variables|Default|GetAKM))
  (|CallParentFunction))