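; A quest Blueprint that sends the player to a Home location, built on a parent quest class.
; It overrides construction of the root objective collection to create an order-required BP_OBJCollection, then populates it with a single "Reach Home" reach-destination objective.
; SetupPOI sets the point-of-interest target to Home before running the parent setup.
; The event graph holds no custom logic beyond calling the parent BeginPlay.
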(event EventBeginPlay
  (|CallParentFunction))

(event Collision|EventActorBeginOverlap
  (params (OtherActor :type Actor%20Object%20Reference))
  (|CallParentFunction OtherActor) ; This node is disabled and will not be called.\nDrag off pins to build functionality.
)

(event EventTick
  (params (DeltaSeconds :type Float%20%28single-precision%29))
  (|CallParentFunction DeltaSeconds) ; This node is disabled and will not be called.\nDrag off pins to build functionality.
)

(fn ConstructionScript
  (|CallParentFunction))

(fn ConstructRootObjectiveCollection
  (bind _self self)
  (bind _returnvalue (Game|ConstructObjectfromClass "/Game/Blueprints/QuestSystem/Objectives/BP_OBJCollection.BP_OBJCollection_C" _self true (Variables|Default|GetObjectiveName) _self))
  (return _returnvalue))

(fn PopulateObjectives
  (params (RootObjectiveCollection :type BP%20OBJ%20Collection%20Object%20Reference))
  (bind _self self)
  (bind _returnvalue (Game|ConstructObjectfromClass "/Game/Blueprints/QuestSystem/Objectives/BP_OBJReachDestination.BP_OBJReachDestination_C" _self (Variables|Default|GetHome) "Reach Home" _self))
  (Default|AddObjective RootObjectiveCollection _returnvalue))

(fn SetupPOI
  (Variables|Default|SetTarget (Variables|Default|GetHome))
  (|CallParentFunction))