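; Base quest actor that manages a quest's active state, objective collection and point-of-interest marker.
; InitializeQuest briefly waits, sets up the POI, then builds and activates the root objective collection only if no quest in the player's QuestManager is active.
; Objective construction and population are placeholders that print errors, apparently for child quests to override.
; Helpers expose the player character, game mode, HUD and quest item actors.
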(event Custom|InitializeQuest
  (Utilities|FlowControl|Delay 0.2)
  (CallFunction|SetupPOI)
  (if (not (CallFunction|IsonGoingQuest))
    (bind _objectcollection (CallFunction|ConstructRootObjectiveCollection))
    (bind _output_get (Variables|Default|SetRootObjectiveCollection _objectcollection))
    (CallFunction|PopulateObjectives _output_get)
    (Default|ActivateObjective (Variables|Default|GetRootObjectiveCollection))
    (CallFunction|ActivateQuest)
    (Development|PrintString "Moving on to next one")))

(event Custom|ActivateQuest
  (Variables|Default|SetIsQuestActive true))

(event EventBeginPlay
  (Variables|Default|SetIsQuestComplete false)
  (Variables|Default|SetIsQuestActive false))

(fn ConstructionScript)

(fn ConstructRootObjectiveCollection
  (Development|PrintString "ErrorFromBP_Quest" true true "(R=0.703125,G=0.036259,B=0.000000,A=1.000000)" 1e+01)
  (return 0))

(fn PopulateObjectives
  (params (RootObjectiveCollection :type BP%20OBJ%20Collection%20Object%20Reference))
  (Development|PrintString "ErrorFromBP_Quest" true true "(R=0.703125,G=0.036259,B=0.000000,A=1.000000)" 1e+01))

(fn GetRootObjectiveCollection
  (return (Variables|Default|GetRootObjectiveCollection)))

(fn IsonGoingQuest
  (bind _asue_4asp_character (Utilities|Casting|CastToUe4ASP_Character (Game|GetPlayerCharacter 0)))
  (for _array_element (Variables|/Game/Blueprints/QuestSystem/Quests/QuestManager.QuestManager_C|GetAllQuests (Variables|/Game/Blueprints/Ue4ASP_Character.Ue4ASP_Character_C|GetQuestManager _asue_4asp_character))
    (if (Variables|BP_Quest_C|GetIsQuestActive _array_element)
      (return true)))
  (return false))

(fn GetPlayerCharacter
  (bind _asue_4asp_character (Utilities|Casting|CastToUe4ASP_Character (Game|GetPlayerCharacter 0)))
  (return _asue_4asp_character))

(fn GetGameMode
  (bind _asbp_shooter_game_mode (Utilities|Casting|CastToBP_ShooterGameMode (Game|GetGameMode)))
  (return _asbp_shooter_game_mode))

(fn GetHUD
  (bind _asbp_in_game_hud (Utilities|Casting|CastToBP_InGameHUD (HUD|GetHUD (Game|GetPlayerController 0))))
  (return _asbp_in_game_hud))

(fn Quest5Helper
  (bind _outactors (Actor|GetAllActorsOfClass "/Game/Blueprints/items/BP_QuestItem1.BP_QuestItem1_C"))
  (return _outactors))

(fn SetupPOI
  (Default|SetupPOIWidget (Variables|Default|GetBP_POIComponent)))

(fn RemovePOI
  (Default|RemovePOI (Variables|Default|GetBP_POIComponent)))