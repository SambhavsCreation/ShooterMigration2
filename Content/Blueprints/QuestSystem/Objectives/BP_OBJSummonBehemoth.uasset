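; Quest objective for summoning a behemoth, completed when the player enters a summoning area while carrying two required item types.
; Activation binds the area's begin-overlap event, which accepts only the player character class and prints a leftover debug string.
; Nested loops search the game mode's inventory for both item types, decrement each quantity by one, then fire the completion call and mark the objective complete.
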(event Custom|OnBeginOverlap
  (params (OverlappedActor :type Actor%20Object%20Reference) (OtherActor :type Actor%20Object%20Reference))
  (bind _ownerquest (Variables|Default|GetOwnerQuest))
  (bind _ownerquest_2 (Variables|Default|GetOwnerQuest))
  (bind _gamemode (Default|GetGameMode _ownerquest))
  (bind _gamemode_2 (Default|GetGameMode _ownerquest_2))
  (bind _inventoryitems (Variables|/Game/Blueprints/BP_ShooterGameMode.BP_ShooterGameMode_C|GetInventoryItems _gamemode))
  (bind _inventoryitems_2 (Variables|/Game/Blueprints/BP_ShooterGameMode.BP_ShooterGameMode_C|GetInventoryItems _gamemode_2))
  (Development|PrintString 0 "why?" true true "(R=0.794169,G=1.000000,B=0.000000,A=1.000000)" 2e+02)
  (bind _asue_4asp_character (Utilities|Casting|CastToUe4ASP_Character OtherActor))
  (for _array_element _inventoryitems_2
    (if (>= (Utilities|Array|FindItem _inventoryitems_2 (Utilities|Struct|MakeInventoryData (.itemclass _array_element) (.isdisplayed _array_element) (.itemname _array_element) (.itemthumbnail _array_element) (.itemquantity _array_element) "NewEnumerator3")) 0)
      (if (> (.itemquantity (Utilities|Array|Get(acopy) _inventoryitems_2 (Utilities|Array|FindItem _inventoryitems_2 (Utilities|Struct|MakeInventoryData (.itemclass _array_element) (.isdisplayed _array_element) (.itemname _array_element) (.itemthumbnail _array_element) (.itemquantity _array_element) "NewEnumerator3")))) 0)
        (for _array_element_2 _inventoryitems
          (if (>= (Utilities|Array|FindItem _inventoryitems (Utilities|Struct|MakeInventoryData (.itemclass _array_element_2) (.isdisplayed _array_element_2) (.itemname _array_element_2) (.itemthumbnail _array_element_2) (.itemquantity _array_element_2) "NewEnumerator4")) 0)
            (if (> (.itemquantity (Utilities|Array|Get(acopy) _inventoryitems (Utilities|Array|FindItem _inventoryitems (Utilities|Struct|MakeInventoryData (.itemclass _array_element_2) (.isdisplayed _array_element_2) (.itemname _array_element_2) (.itemthumbnail _array_element_2) (.itemquantity _array_element_2) "NewEnumerator4")))) 0)
              (Utilities|Array|SetArrayElem _inventoryitems_2 (Utilities|Array|FindItem _inventoryitems_2 (Utilities|Struct|MakeInventoryData (.itemclass _array_element) (.isdisplayed _array_element) (.itemname _array_element) (.itemthumbnail _array_element) (.itemquantity _array_element) "NewEnumerator3")) (Utilities|Struct|MakeInventoryData (.itemclass (Utilities|Array|Get(acopy) _inventoryitems_2 (Utilities|Array|FindItem _inventoryitems_2 (Utilities|Struct|MakeInventoryData (.itemclass _array_element) (.isdisplayed _array_element) (.itemname _array_element) (.itemthumbnail _array_element) (.itemquantity _array_element) "NewEnumerator3")))) (.isdisplayed (Utilities|Array|Get(acopy) _inventoryitems_2 (Utilities|Array|FindItem _inventoryitems_2 (Utilities|Struct|MakeInventoryData (.itemclass _array_element) (.isdisplayed _array_element) (.itemname _array_element) (.itemthumbnail _array_element) (.itemquantity _array_element) "NewEnumerator3")))) (.itemname (Utilities|Array|Get(acopy) _inventoryitems_2 (Utilities|Array|FindItem _inventoryitems_2 (Utilities|Struct|MakeInventoryData (.itemclass _array_element) (.isdisplayed _array_element) (.itemname _array_element) (.itemthumbnail _array_element) (.itemquantity _array_element) "NewEnumerator3")))) (.itemthumbnail (Utilities|Array|Get(acopy) _inventoryitems_2 (Utilities|Array|FindItem _inventoryitems_2 (Utilities|Struct|MakeInventoryData (.itemclass _array_element) (.isdisplayed _array_element) (.itemname _array_element) (.itemthumbnail _array_element) (.itemquantity _array_element) "NewEnumerator3")))) (- (.itemquantity (Utilities|Array|Get(acopy) _inventoryitems_2 (Utilities|Array|FindItem _inventoryitems_2 (Utilities|Struct|MakeInventoryData (.itemclass _array_element) (.isdisplayed _array_element) (.itemname _array_element) (.itemthumbnail _array_element) (.itemquantity _array_element) "NewEnumerator3")))) 1) "NewEnumerator3"))
              (Utilities|Array|SetArrayElem _inventoryitems_2 (Utilities|Array|FindItem _inventoryitems (Utilities|Struct|MakeInventoryData (.itemclass _array_element_2) (.isdisplayed _array_element_2) (.itemname _array_element_2) (.itemthumbnail _array_element_2) (.itemquantity _array_element_2) "NewEnumerator4")) (Utilities|Struct|MakeInventoryData (.itemclass (Utilities|Array|Get(acopy) _inventoryitems (Utilities|Array|FindItem _inventoryitems (Utilities|Struct|MakeInventoryData (.itemclass _array_element_2) (.isdisplayed _array_element_2) (.itemname _array_element_2) (.itemthumbnail _array_element_2) (.itemquantity _array_element_2) "NewEnumerator4")))) (.isdisplayed (Utilities|Array|Get(acopy) _inventoryitems (Utilities|Array|FindItem _inventoryitems (Utilities|Struct|MakeInventoryData (.itemclass _array_element_2) (.isdisplayed _array_element_2) (.itemname _array_element_2) (.itemthumbnail _array_element_2) (.itemquantity _array_element_2) "NewEnumerator4")))) (.itemname (Utilities|Array|Get(acopy) _inventoryitems (Utilities|Array|FindItem _inventoryitems (Utilities|Struct|MakeInventoryData (.itemclass _array_element_2) (.isdisplayed _array_element_2) (.itemname _array_element_2) (.itemthumbnail _array_element_2) (.itemquantity _array_element_2) "NewEnumerator4")))) (.itemthumbnail (Utilities|Array|Get(acopy) _inventoryitems (Utilities|Array|FindItem _inventoryitems (Utilities|Struct|MakeInventoryData (.itemclass _array_element_2) (.isdisplayed _array_element_2) (.itemname _array_element_2) (.itemthumbnail _array_element_2) (.itemquantity _array_element_2) "NewEnumerator4")))) (- (.itemquantity (Utilities|Array|Get(acopy) _inventoryitems (Utilities|Array|FindItem _inventoryitems (Utilities|Struct|MakeInventoryData (.itemclass _array_element_2) (.isdisplayed _array_element_2) (.itemname _array_element_2) (.itemthumbnail _array_element_2) (.itemquantity _array_element_2) "NewEnumerator4")))) 1) "NewEnumerator4"))
              (Default|CallOnCompleted self _asue_4asp_character)
              (Variables|Default|SetIsActive false)
              (Variables|Default|SetIsComplete true))))))))

(event EventActivateObjective
  (|CallParentFunction)
  (Collision|BindEventtoOnActorBeginOverlap (Variables|Default|GetSummoningArea) (delegate Custom|OnBeginOverlap)))

(fn GetIsComplete
  (return (Variables|Default|GetIsComplete)))