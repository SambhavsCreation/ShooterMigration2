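; Quest objective Blueprint that completes when the player picks up the AKM rifle.
; On activation it calls the parent logic and binds to the AKM rifle's quest-complete event.
; When that event fires, it prints a debug message, broadcasts completion with the owning quest's player character, and marks itself inactive and complete.
; An override exposes the completion flag.
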(event Custom|OnItemPicked
  (Development|PrintString 0 "PickUpAKMQuestComplete" true true "(R=0.000000,G=0.089375,B=0.135417,A=1.000000)" 2e+01)
  (Default|CallOnCompleted self (Default|GetPlayerCharacter (Variables|Default|GetOwnerQuest)))
  (Variables|Default|SetIsActive false)
  (Variables|Default|SetIsComplete true))

(event EventActivateObjective
  (|CallParentFunction)
  (EventDispatchers|BindEventtoOnQuestComplete (Variables|Default|GetAKMRifle) (delegate Custom|OnItemPicked)))

(fn GetIsComplete
  (return (Variables|Default|GetIsComplete)))