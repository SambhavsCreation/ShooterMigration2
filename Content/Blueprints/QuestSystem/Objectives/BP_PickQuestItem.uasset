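; Quest objective that completes when the player picks up its bound quest item.
; On activation it binds to the item's picked event, which fires the completion callback with the player and marks the objective inactive and complete.
; A separate completion check scans the game mode's inventory for any entry of a fixed enum type with a positive quantity, rather than comparing against the bound item.
; Both paths print debug messages.
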(event Custom|OnItemPicked
  (Development|PrintString 0 "PickItemQuestCompleted" true true "(R=0.000000,G=0.089375,B=0.135417,A=1.000000)" 2e+01)
  (Default|CallOnCompleted self (Default|GetPlayerCharacter (Variables|Default|GetOwnerQuest)))
  (Variables|Default|SetIsActive false)
  (Variables|Default|SetIsComplete true))

(event EventActivateObjective
  (|CallParentFunction)
  (EventDispatchers|BindEventtoOnQuestItemPicked (Variables|Default|GetQuestItem) (delegate Custom|OnItemPicked)))

(fn GetIsComplete
  (bind _ownerquest (Variables|Default|GetOwnerQuest))
  (bind _gamemode (Default|GetGameMode _ownerquest))
  (bind _inventoryitems (Variables|/Game/Blueprints/BP_ShooterGameMode.BP_ShooterGameMode_C|GetInventoryItems _gamemode))
  (for _array_element _inventoryitems
    (if (>= (Utilities|Array|FindItem _inventoryitems (Utilities|Struct|MakeInventoryData (.itemclass _array_element) (.isdisplayed _array_element) (.itemname _array_element) (.itemthumbnail _array_element) (.itemquantity _array_element) "NewEnumerator3")) 0)
      (if (> (.itemquantity (Utilities|Array|Get(acopy) _inventoryitems (Utilities|Array|FindItem _inventoryitems (Utilities|Struct|MakeInventoryData (.itemclass _array_element) (.isdisplayed _array_element) (.itemname _array_element) (.itemthumbnail _array_element) (.itemquantity _array_element) "NewEnumerator3")))) 0)
        (Development|PrintString 0 "FoundIt!")
        (Development|PrintString 0 (Utilities|String|ToString(Integer) (Utilities|Array|FindItem _inventoryitems (Utilities|Struct|MakeInventoryData (.itemclass _array_element) (.isdisplayed _array_element) (.itemname _array_element) (.itemthumbnail _array_element) (.itemquantity _array_element) "NewEnumerator3"))))
        (return true))))
  (return false))