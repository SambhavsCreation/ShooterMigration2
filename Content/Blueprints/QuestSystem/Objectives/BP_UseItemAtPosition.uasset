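; Quest objective that completes when the player uses an item while at a target location.
; OnUseItemAtLocation searches the game mode's inventory for a matching entry with positive quantity, then marks the objective complete and fires completion if WasSuccessful is set.
; Overlap handlers set or clear WasSuccessful for the player character, but their binding to LocationToUseAt is disconnected.
; Debug prints trace each stage.
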(event Custom|OnUseItemAtLocation
  (bind _ownerquest (Variables|Default|GetOwnerQuest))
  (bind _gamemode (Default|GetGameMode _ownerquest))
  (bind _inventoryitems (Variables|/Game/Blueprints/BP_ShooterGameMode.BP_ShooterGameMode_C|GetInventoryItems _gamemode))
  (Development|PrintString 0 "chalo" true true "(R=0.000000,G=0.660000,B=1.000000,A=1.000000)" 3e+01)
  (for _array_element _inventoryitems
    (if (>= (Utilities|Array|FindItem _inventoryitems (Utilities|Struct|MakeInventoryData (.itemclass _array_element) (.isdisplayed _array_element) (.itemname _array_element) (.itemthumbnail _array_element) (.itemquantity _array_element) "NewEnumerator3")) 0)
      (Development|PrintString 0 "idk")
      (if (> (.itemquantity (Utilities|Array|Get(acopy) _inventoryitems (Utilities|Array|FindItem _inventoryitems (Utilities|Struct|MakeInventoryData (.itemclass _array_element) (.isdisplayed _array_element) (.itemname _array_element) (.itemthumbnail _array_element) (.itemquantity _array_element) "NewEnumerator3")))) 0)
        (if (Variables|Default|GetWasSuccessful)
          (Development|PrintString 0 "EZ NOOBS" true true "(R=0.997782,G=1.000000,B=0.000000,A=1.000000)" 1.2e+02)
          (Development|PrintString 0 "UseItemQuestCompleted" true true "(R=0.000000,G=0.089375,B=0.135417,A=1.000000)" 2e+01)
          (Default|CallOnCompleted self (Default|GetPlayerCharacter (Variables|Default|GetOwnerQuest)))
          (Variables|Default|SetIsActive false)
          (Variables|Default|SetIsComplete true))))))

(event Custom|OnActorBeginOverlap
  (params (OverlappedActor :type Actor%20Object%20Reference) (OtherActor :type Actor%20Object%20Reference))
  (Utilities|Casting|CastToUe4ASP_Character OtherActor
    (:then
      (Variables|Default|SetWasSuccessful true)
      (Development|PrintString 0 "shud bork irl"))
    (:CastFailed
      (Variables|Default|SetWasSuccessful false))))

(event Custom|OnActorEndOverlap_Event_0
  (params (OverlappedActor :type Actor%20Object%20Reference) (OtherActor :type Actor%20Object%20Reference))
  (Variables|Default|SetWasSuccessful false)
  (Development|PrintString 0 "tu bhi"))

(event EventActivateObjective
  (|CallParentFunction))

(fn GetIsComplete
  (return (Variables|Default|GetIsComplete)))

(fn GetIsatLocation
  (return (Variables|Default|GetWasSuccessful)))