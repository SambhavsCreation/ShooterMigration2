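; BP_POIComponent is a component that marks its owning actor as a point of interest on the minimap.
; SetupPOIWidget reaches the minimap through the first player's BP_InGameHUD and main interface widget, adds a POI for the owner and stores the returned widget.
; RemovePOI removes that stored widget from its parent.
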(fn SetupPOIWidget
  (bind _asbp_in_game_hud (Utilities|Casting|CastToBP_InGameHUD (HUD|GetHUD (Game|GetPlayerController 0))))
  (bind _createdwidget (Default|AddPOI (Variables|/Game/Blueprints/WBP_Interface.WBP_Interface_C|GetMinimap (Variables|/Game/Blueprints/BP_InGameHUD.BP_InGameHUD_C|GetMainInterfaceWidget _asbp_in_game_hud)) (Components|GetOwner)))
  (Variables|Default|SetThisPOIWidget _createdwidget))

(fn RemovePOI
  (Widget|RemovefromParent (Variables|Default|GetThisPOIWidget)))