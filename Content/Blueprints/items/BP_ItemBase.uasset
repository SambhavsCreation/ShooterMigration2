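; BP_ItemBase is a base item Blueprint that handles the interaction-range prompt and use from the inventory.
; Entering range lazily creates a WBP_ItemOverlapAlert for the player, then reuses it by toggling visibility on exit and re-entry.
; Inventory use decrements the slot's quantity in BP_ShooterGameMode's InventoryItems, prints it for debugging and refreshes BP_InGameHUD.
; It applies no item effect and has no zero-quantity check.
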(event EventBeginPlay)

(event Collision|EventActorBeginOverlap
  (params (OtherActor :type Actor%20Object%20Reference)))

(event EventTick
  (params (DeltaSeconds :type Float%20%28single-precision%29)))

(event EventInteractionRangeExited
  (bind _overlapwidget (Variables|Default|GetOverlapWidget)
    (:then
      (Widget|SetVisibility _overlapwidget "Hidden"))
    (:else)))

(event EventInteractionRangeEntered
  (params (Player :type Ue%204ASP%20Character%20Object%20Reference))
  (Variables|Default|GetOverlapWidget
    (:then
      (Widget|SetVisibility (Variables|Default|GetOverlapWidget) "Visible"))
    (:else
      (bind _asplayer_controller (Utilities|Casting|CastToPlayerController (Pawn|GetController Player)))
      (bind _returnvalue (UserInterface|CreateWidget "/Game/Blueprints/WBP_ItemOverlapAlert.WBP_ItemOverlapAlert_C" _asplayer_controller))
      (bind _output_get (Variables|Default|SetOverlapWidget _returnvalue))
      (UserInterface|Viewport|AddtoViewport _output_get 0))))

(fn ConstructionScript)

(fn OnUsefromInventoryButton
  (params (SlotID :type Integer))
  (Variables|Default|SetItemSlot SlotID)
  (bind _asbp_shooter_game_mode (Utilities|Casting|CastToBP_ShooterGameMode (Game|GetGameMode)))
  (bind _output_get (Variables|Default|SetTempData (Utilities|Array|Get(acopy) (Variables|/Game/Blueprints/BP_ShooterGameMode.BP_ShooterGameMode_C|GetInventoryItems _asbp_shooter_game_mode) SlotID)))
  (bind _output_get_2 (Variables|Default|SetTempData (Utilities|Struct|MakeInventoryData (.itemclass _output_get) (.isdisplayed _output_get) (.itemname _output_get) (.itemthumbnail _output_get) (- (.itemquantity _output_get) 1) (.itemtype _output_get))))
  (Utilities|Array|SetArrayElem (Variables|/Game/Blueprints/BP_ShooterGameMode.BP_ShooterGameMode_C|GetInventoryItems _asbp_shooter_game_mode) SlotID _output_get_2)
  (Development|PrintString "Quantity" true true "(R=1.000000,G=0.000000,B=0.076232,A=1.000000)" 22.0)
  (Development|PrintString (Utilities|String|ToString(Integer) (.itemquantity _output_get)) true true "(R=1.000000,G=0.000000,B=0.076232,A=1.000000)" 22.0)
  (bind _asbp_in_game_hud (Utilities|Casting|CastToBP_InGameHUD (HUD|GetHUD (Game|GetPlayerController 0))))
  (Default|RefreshWidget _asbp_in_game_hud))