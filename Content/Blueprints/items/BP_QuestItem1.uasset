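; BP_QuestItem1 is a quest pickup that is later used from the inventory at a location required by BP_Quest_5.
; Interaction broadcasts the pickup, hides the item, disables its collision, adds it to the game mode and refreshes the HUD.
; Inventory use fires a self-bound dispatcher that finds BP_Quest_5 in the player's QuestManager and notifies its objective if at location.
; The resulting IsSuccessful flag gates the parent's use logic.
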(event Custom|CustomEvent_0
  (bind _asue_4asp_character (Utilities|Casting|CastToUe4ASP_Character (Game|GetPlayerCharacter 0)))
  (for _array_element (Variables|/Game/Blueprints/QuestSystem/Quests/QuestManager.QuestManager_C|GetAllQuests (Variables|/Game/Blueprints/Ue4ASP_Character.Ue4ASP_Character_C|GetQuestManager _asue_4asp_character))
    (if (== (Utilities|GetClass _array_element) "/Game/Blueprints/QuestSystem/Quests/BP_Quest_5.BP_Quest_5_C")
      (bind _asbp_quest_5 (Utilities|Casting|CastToBP_Quest_5 _array_element))
      (bind _output_get (Variables|Default|SetQuest5BP _asbp_quest_5))
      (bind _isatlocation (Default|GetIsatLocation (Variables|/Game/Blueprints/QuestSystem/Quests/BP_Quest_5.BP_Quest_5_C|GetObjective _output_get)))
      (Variables|Default|SetIsSuccessful _isatlocation)
      (if _isatlocation
        (Default|OnUseItematLocation (Variables|/Game/Blueprints/QuestSystem/Quests/BP_Quest_5.BP_Quest_5_C|GetObjective _output_get))))))

(event Collision|EventActorBeginOverlap
  (params (OtherActor :type Actor%20Object%20Reference))
  (|CallParentFunction OtherActor) ; This node is disabled and will not be called.\nDrag off pins to build functionality.
)

(event EventTick
  (params (DeltaSeconds :type Float%20%28single-precision%29))
  (|CallParentFunction DeltaSeconds) ; This node is disabled and will not be called.\nDrag off pins to build functionality.
)

(event EventOnInteracted
  (params (Player :type Ue%204ASP%20Character%20Object%20Reference))
  (Default|CallOnQuestItemPicked)
  (Rendering|SetVisibility (Variables|Default|Getr) false false)
  (Collision|SetCollisionEnabled (Variables|Default|GetSphere) "NoCollision")
  (bind _asbp_shooter_game_mode (Utilities|Casting|CastToBP_ShooterGameMode (Game|GetGameMode)))
  (Default|AddItem _asbp_shooter_game_mode (Variables|Default|GetThisItemType))
  (bind _asbp_in_game_hud (Utilities|Casting|CastToBP_InGameHUD (HUD|GetHUD (Game|GetPlayerController 0))))
  (Default|RefreshWidget _asbp_in_game_hud))

(event EventBeginPlay
  (EventDispatchers|BindEventtoUseItematLocation (delegate Custom|CustomEvent_0)))

(fn ConstructionScript
  (|CallParentFunction))

(fn OnUsefromInventoryButton
  (params (SlotID :type Integer))
  (Default|CallUseItematLocation)
  (if (Variables|Default|GetIsSuccessful)
    (|CallParentFunction SlotID)))