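; BP_SummoningArtifact1 is an interactable summoning artifact pickup that notifies the quest system and enters the player's inventory.
; On interaction it fires the quest-item-picked call, destroys itself, then adds its item type through BP_ShooterGameMode and refreshes the BP_InGameHUD widget.
; Its use-from-inventory function is empty, so using it from a slot does nothing here.
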(event EventBeginPlay)

(event Collision|EventActorBeginOverlap
  (params (OtherActor :type Actor%20Object%20Reference)))

(event EventTick
  (params (DeltaSeconds :type Float%20%28single-precision%29)))

(event EventOnInteracted
  (params (Player :type Ue%204ASP%20Character%20Object%20Reference))
  (Default|CallOnQuestItemPicked)
  (Actor|DestroyActor)
  (bind _asbp_shooter_game_mode (Utilities|Casting|CastToBP_ShooterGameMode (Game|GetGameMode)))
  (Default|AddItem _asbp_shooter_game_mode (Variables|Default|GetThisItemType))
  (bind _asbp_in_game_hud (Utilities|Casting|CastToBP_InGameHUD (HUD|GetHUD (Game|GetPlayerController 0))))
  (Default|RefreshWidget _asbp_in_game_hud))

(fn ConstructionScript
  (|CallParentFunction))

(fn OnUsefromInventoryButton
  (params (SlotID :type Integer)))