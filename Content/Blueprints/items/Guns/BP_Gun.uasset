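; Gun item that the player picks up, fires, reloads and throws, tracking magazine and reserve ammo.
; Pickup and throw replace the actor with a new one of the same class, copying ammo and switching collision: socket-attached when held, physics-simulated when dropped.
; Fire decrements the magazine and runs a debug-drawn camera line trace without applying hits.
; Reload moves reserve rounds into the magazine up to a hard-coded capacity.
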(event EventBeginPlay
  (Variables|Default|SetBulletsInCurrentMagazine (Variables|Default|GetBulletsPerMagazine)))

(event EventOnThrowTriggered
  (params (Player :type Ue%204ASP%20Character%20Object%20Reference))
  (bind _gun (Variables|/Game/Blueprints/Ue4ASP_Character.Ue4ASP_Character_C|GetGun Player))
  (Development|PrintString "throw revoked")
  (Utilities|IsValid _gun
    (:Is%20Valid
      (bind _output_get (Variables|Default|SetBICMTemp (Variables|BP_Gun_C|GetBulletsInCurrentMagazine _gun)))
      (Variables|Default|SetTCATemp (Variables|BP_Gun_C|GetTotalCurrentAmmo _gun))
      (Development|PrintString (Utilities|String|ToString(Integer) _output_get))
      (Actor|DestroyActor)
      (Development|PrintString "delactor")
      (bind _returnvalue (Game|SpawnActorfromClass (Utilities|GetClass _gun) (Math|Transform|MakeTransform (Transformation|GetActorLocation)) "Undefined" 0 0))
      (bind _output_get_2 (Variables|BP_Gun_C|SetBulletsInCurrentMagazine _returnvalue (Variables|Default|GetBICMTemp)))
      (Development|PrintString (Utilities|String|ToString(Integer) _output_get_2))
      (Variables|BP_Gun_C|SetTotalCurrentAmmo _returnvalue (Variables|Default|GetTCATemp))
      (Collision|SetCollisionProfileName (Variables|BP_Gun_C|GetSphere _returnvalue) "OverlapAllDynamic" true :!class /Script/Engine.PrimitiveComponent)
      (Collision|SetCollisionProfileName (Variables|BP_Gun_C|GetSkeletalMesh _returnvalue) "DroppedGun" true :!class /Script/Engine.PrimitiveComponent)
      (Physics|SetSimulatePhysics (Variables|BP_Gun_C|GetSkeletalMesh _returnvalue) true))))

(event EventOnInteracted
  (params (Player :type Ue%204ASP%20Character%20Object%20Reference))
  (Utilities|IsValid (Variables|/Game/Blueprints/Ue4ASP_Character.Ue4ASP_Character_C|GetGun Player)
    (:Is%20Not%20Valid
      (bind _returnvalue (Game|SpawnActorfromClass (Utilities|GetClass self) (Math|Transform|MakeTransform "0, 0, 0") "Undefined" 0 0))
      (bind _output_get (Variables|/Game/Blueprints/Ue4ASP_Character.Ue4ASP_Character_C|SetGun Player _returnvalue))
      (Collision|SetCollisionProfileName (Variables|BP_Gun_C|GetSkeletalMesh _output_get) "NoCollision" true :!class /Script/Engine.PrimitiveComponent)
      (Collision|SetCollisionProfileName (Variables|BP_Gun_C|GetSphere _output_get) "NoCollision" true :!class /Script/Engine.PrimitiveComponent)
      (Variables|BP_Gun_C|SetBulletsInCurrentMagazine _output_get (Variables|Default|GetBulletsInCurrentMagazine))
      (Development|PrintString (Utilities|String|ToString(Integer) 0))
      (Variables|BP_Gun_C|SetTotalCurrentAmmo _output_get (Variables|Default|GetTotalCurrentAmmo))
      (Transformation|AttachComponentToComponent _output_get (Variables|/Script/Engine.Character|GetMesh Player) "WeaponSocket" "KeepRelative" "KeepRelative" "KeepRelative" true)
      (Actor|DestroyActor))))

(fn ConstructionScript
  (|CallParentFunction))

(fn Fire
  (if (and (< (Variables|Default|GetBulletsInCurrentMagazine) 0) (< (Variables|Default|GetTotalCurrentAmmo) 0))
    (Variables|Default|SetCanNotFire true)
    (return)
    (else
      (Variables|Default|SetBulletsInCurrentMagazine (- (Variables|Default|GetBulletsInCurrentMagazine) 1))
      (bind _asue_4asp_character (Utilities|Casting|CastToUe4ASP_Character (Game|GetPlayerCharacter 0)))
      (Collision|LineTraceByChannel (Transformation|GetWorldLocation (Variables|/Game/Blueprints/Ue4ASP_Character.Ue4ASP_Character_C|GetPlayerCamera _asue_4asp_character)) (+ (Transformation|GetWorldLocation (Variables|/Game/Blueprints/Ue4ASP_Character.Ue4ASP_Character_C|GetPlayerCamera _asue_4asp_character)) (* (Math|Vector|GetForwardVector (Transformation|GetWorldRotation (Variables|/Game/Blueprints/Ue4ASP_Character.Ue4ASP_Character_C|GetPlayerCamera _asue_4asp_character))) 1.5e+03)) "TraceTypeQuery1" false 0 "Persistent"))))

(fn ReloadGun
  (if (> (Variables|Default|GetTotalCurrentAmmo) 0)
    (if (== (Variables|Default|GetBulletsInCurrentMagazine) 30)
      (return)
      (else
        (Utilities|FlowControl|ForLoopwithBreak (Variables|Default|GetBulletsInCurrentMagazine) 30
          (:LoopBody
            (if (> (Variables|Default|GetTotalCurrentAmmo) 0)
              (Variables|Default|SetBulletsInCurrentMagazine (+ (Variables|Default|GetBulletsInCurrentMagazine) 1))
              (Variables|Default|SetTotalCurrentAmmo (- (Variables|Default|GetTotalCurrentAmmo) 1))
              (if (== (Variables|Default|GetBulletsInCurrentMagazine) 30)
                (return))
              (else
                (return)))))))
    (else
      (return))))