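; Health potion pickable that goes into the inventory and restores player health when used from there.
; On interaction it destroys itself, adds its item type through BP_ShooterGameMode and refreshes the BP_InGameHUD widget.
; Using it from an inventory button adds HealthToIncrease to the Ue4ASP_Character's Health without clamping, then calls the parent handler with slot 0 instead of the received SlotID.
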(event EventBeginPlay
  (|CallParentFunction) ; This node is disabled and will not be called.\nDrag off pins to build functionality.
)

(event Collision|EventActorBeginOverlap
  (params (OtherActor :type Actor%20Object%20Reference))
  (|CallParentFunction OtherActor) ; This node is disabled and will not be called.\nDrag off pins to build functionality.
)

(event EventTick
  (params (DeltaSeconds :type Float%20%28single-precision%29)))

(event EventOnInteracted
  (params (Player :type Ue%204ASP%20Character%20Object%20Reference))
  (Actor|DestroyActor)
  (bind _asbp_shooter_game_mode (Utilities|Casting|CastToBP_ShooterGameMode (Game|GetGameMode)))
  (Default|AddItem _asbp_shooter_game_mode (Variables|Default|GetThisItemType))
  (bind _asbp_in_game_hud (Utilities|Casting|CastToBP_InGameHUD (HUD|GetHUD (Game|GetPlayerController 0))))
  (Default|RefreshWidget _asbp_in_game_hud))

(fn ConstructionScript
  (|CallParentFunction))

(fn OnUsefromInventoryButton
  (params (SlotID :type Integer))
  (Development|PrintString "Health Potion here")
  (bind _asue_4asp_character (Utilities|Casting|CastToUe4ASP_Character (Game|GetPlayerCharacter 0)))
  (Variables|/Game/Blueprints/Ue4ASP_Character.Ue4ASP_Character_C|SetHealth _asue_4asp_character (+ (Variables|/Game/Blueprints/Ue4ASP_Character.Ue4ASP_Character_C|GetHealth _asue_4asp_character) (Variables|Default|GetHealthToIncrease)))
  (|CallParentFunction 0))