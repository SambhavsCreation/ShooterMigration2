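; BP_AmmuntionPickable is an ammo pickup that adds a fixed amount of ammo to the interacting player's gun.
; OnInteracted increases the gun's TotalCurrentAmmo and destroys the actor, or prints "Find a weapon" when the player has no gun.
; InteractionRangeEntered shows a WBP_ItemOverlapAlert to armed players only, creating the widget once and reusing it afterwards.
; Nothing in this graph hides or removes that widget.
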(event EventBeginPlay
  (|CallParentFunction) ; This node is disabled and will not be called.\nDrag off pins to build functionality.
)

(event Collision|EventActorBeginOverlap
  (params (OtherActor :type Actor%20Object%20Reference))
  (|CallParentFunction OtherActor) ; This node is disabled and will not be called.\nDrag off pins to build functionality.
)

(event EventOnInteracted
  (params (Player :type Ue%204ASP%20Character%20Object%20Reference))
  (bind _gun (Variables|/Game/Blueprints/Ue4ASP_Character.Ue4ASP_Character_C|GetGun Player))
  (Development|PrintString "valid")
  (Utilities|IsValid _gun
    (:Is%20Valid
      (Variables|/Game/Blueprints/items/Guns/BP_Gun.BP_Gun_C|SetTotalCurrentAmmo _gun (+ (Variables|/Game/Blueprints/items/Guns/BP_Gun.BP_Gun_C|GetTotalCurrentAmmo _gun) 30))
      (Actor|DestroyActor))
    (:Is%20Not%20Valid
      (Development|PrintString "Find a weapon"))))

(event EventInteractionRangeEntered
  (params (Player :type Ue%204ASP%20Character%20Object%20Reference))
  (Utilities|IsValid (Variables|/Game/Blueprints/Ue4ASP_Character.Ue4ASP_Character_C|GetGun Player)
    (:Is%20Valid
      (Variables|Default|GetOverlapWidget
        (:then
          (Widget|SetVisibility (Variables|Default|GetOverlapWidget) "Visible"))
        (:else
          (bind _asplayer_controller (Utilities|Casting|CastToPlayerController (Pawn|GetController Player)))
          (bind _returnvalue (UserInterface|CreateWidget "/Game/Blueprints/Inventory/UI/WBP_ItemOverlapAlert.WBP_ItemOverlapAlert_C" _asplayer_controller))
          (bind _output_get (Variables|Default|SetOverlapWidget _returnvalue))
          (UserInterface|Viewport|AddtoViewport _output_get 0))))))

(fn ConstructionScript
  (|CallParentFunction))